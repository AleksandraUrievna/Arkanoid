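; Game mode for a ball-and-blocks game that tracks lives, score, remaining blocks and game state.
; BeginPlay creates the HUD widget and resets the game, calling ResetPlayerPosition and StartGame.
; Score, lost-ball and block-count events update the widget directly, clamping score and blocks at zero and penalizing lost balls.
; Losing the last ball or clearing all blocks sets an end state, adds an audio component, then opens MainMenu after a delay.
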(event `self.ReceiveBeginPlay`
  ;[1 1 1] Add GUI
  (bind _returnvalue (`|CreateWidget` "/Game/UI/GUI.GUI_C"))
  (bind _output_get (set `self.GUI` _returnvalue))
  (`UserWidget.AddToViewport` _output_get 0)
  (`self.Reset Game`))

(event `Reset Game`
  (bind _score (`self.Score`))
  (bind _maxlifes (`self.MaxLifes`))
  (bind _gui (`self.GUI`))
  ;[1 1 1] Reset Game
  (set `self.CurrentBall` _maxlifes)
  (set `/Game/UI/GUI.Balls Left` _maxlifes _gui)
  (set `/Game/UI/GUI.Score` _score _gui)
  (set `self.CurrentScore` _score)
  (set `self.CurretBlocks` (`self.NewBlocks`))
  (`self.ResetPlayerPosition`)
  (set `self.EGameState` "NewEnumerator0")
  (`self.StartGame`))

(event `UpdataScore`
  (params (Points :type "Float (double-precision)" :default 0.0))
  (bind _returnvalue (+ Points (`self.CurrentScore`)))
  ;[1 1 1] Update Score
  (if (< _returnvalue 0.0)
    (set `self.CurrentScore` 0.0)
    (else
      (set `self.CurrentScore` _returnvalue)))
  (set `/Game/UI/GUI.Score` (`self.CurrentScore`) (`self.GUI`)))

(event `LostBall`
  (bind _currentball (`self.CurrentBall`))
  ;[1 1 1] Ball Lost
  (`self.UpdataScore` -1000.0)
  (if (<= _currentball 1.0)
    (`self.GameOver`)
    (else
      (bind _output_get (set `self.CurrentBall` (- _currentball 1.0)))
      (set `/Game/UI/GUI.Balls Left` _output_get (`self.GUI`)))))

(event `GameOver`
  ;[1 1 1] Game Over
  (set `self.EGameState` "NewEnumerator1")
  (`AddComponent|NODE_AddAudioComponent-1`)
  (`KismetSystemLibrary.Delay` 4.0)
  (`GameplayStatics.OpenLevel` "MainMenu"))

(event `UpdataBlock`
  (params (Counter :type "Float (double-precision)" :default 0.0))
  (bind _returnvalue (- (`self.CurretBlocks`) Counter))
  ;[1 1 1] Block Updata
  (if (< _returnvalue 0.0)
    (set `self.CurretBlocks` 0.0)
    (else
      (set `self.CurretBlocks` _returnvalue)))
  (bind _output_get (set `/Game/UI/GUI.Blocks` (`self.CurretBlocks`) (`self.GUI`)))
  (if (== _output_get 0.0)
    (set `self.EGameState` "NewEnumerator2")
    (`AddComponent|NODE_AddAudioComponent-2`)
    (`KismetSystemLibrary.Delay` 5.0)
    (`GameplayStatics.OpenLevel` "MainMenu")))

(fn `UserConstructionScript`)