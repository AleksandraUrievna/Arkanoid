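; Player pawn for a paddle-and-ball game that moves the paddle, launches the ball and returns to the main menu on exit.
; It spawns Ball_BP at an Arrow component and launches it along that arrow, while horizontal input pushes the paddle with physics impulses.
; Game mode events trigger ball respawns and position resets, and its state gates spawning and movement.
; Holding Acceleration multiplies ball speed, with a threshold check before reverting on release.
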(event `self.ReceiveBeginPlay`
  (bind _gamemode (`self.GameMode`))
  ;[1 1 1] Get Game Mode
  (bind _asmy_game_mode (cast `/Game/Blueprints/MyGameMode` (`GameplayStatics.GetGameMode`)))
  (set `self.GameMode` _asmy_game_mode)
  (`self.Spawn New Ball`)
  ;[1 1 1] Save Player Start Location
  (set `self.PlayerStartLocation` (`self.K2_GetActorLocation`))
  ;[1 1 1] Bind Events
  (add `/Game/Blueprints/MyGameMode.ResetPlayerPosition` _gamemode (delegate `ResetPlayerPosition`))
  (add `/Game/Blueprints/MyGameMode.StartGame` _gamemode (delegate `Spawn New Ball`)))

(event `ResetPlayerPosition`
  (bind _playerstartlocation (`self.PlayerStartLocation`))
  ;[1 1 1] Reset Player Position
  (`self.K2_SetActorLocation` _playerstartlocation)
  (`SceneComponent.K2_SetWorldLocation` (`self.Paddle`) _playerstartlocation false false))

(event `Spawn New Ball`
  ;[1 1 1] Spawn New Ball
  (if (`|EnumEquality` (`/Game/Blueprints/MyGameMode.EGameState` (`self.GameMode`)) "NewEnumerator0")
    (bind _returnvalue (`|SpawnActorFromClass` "/Game/Blueprints/Ball_BP.Ball_BP_C" (`SceneComponent.K2_GetComponentToWorld` (`self.Arrow`)) "AlwaysSpawn" "OverrideRootScale" null null))
    (set `self.Ball` _returnvalue)))

(event `InputAxis|MoveHorizontal`
  (params (AxisValue :type "Float (single-precision)"))
  ;[1 1 1] Movement
  (`/Engine/EditorBlueprintResources/StandardMacros.IsValid` (`self.Ball`)
    (:`Is Valid`
      (if (`|EnumEquality` (`/Game/Blueprints/MyGameMode.EGameState` (`self.GameMode`)) "NewEnumerator0")
        (`PrimitiveComponent.AddImpulse` (`self.Paddle`) (`KismetMathLibrary.MakeVector` (* AxisValue (`self.Speed`))) "None" false)))))

(event `InputAction|Fire`
  (params (Key :type "Key Structure"))
  (bind _ball (`self.Ball`))
  ;[1 1 1] Launch Ball
  (:`Pressed`
    (`/Engine/EditorBlueprintResources/StandardMacros.IsValid` _ball
      (:`Is Valid`
        (if (not (`/Game/Blueprints/Ball_BP.Active` _ball))
          (`/Game/Blueprints/Ball_BP.Launch` _ball (`KismetMathLibrary.Conv_RotatorToVector` (`SceneComponent.K2_GetComponentRotation` (`self.Arrow`)))))))))

(event `InputAction|Acceleration`
  (params (Key :type "Key Structure"))
  (bind _ball (`self.Ball`))
  (bind _ball_2 (`self.Ball`))
  (bind _speed (`/Game/Blueprints/Ball_BP.Speed` _ball_2))
  ;[1 1 1] Acceleration
  (:`Pressed`
    (`/Engine/EditorBlueprintResources/StandardMacros.IsValid` _ball
      (:`Is Valid`
        (set `/Game/Blueprints/Ball_BP.Speed` (* (`/Game/Blueprints/Ball_BP.Speed` _ball) 1.75) _ball))))
  (:`Released`
    (`/Engine/EditorBlueprintResources/StandardMacros.IsValid` _ball_2
      (:`Is Valid`
        (if (> _speed 290.0)
          (set `/Game/Blueprints/Ball_BP.Speed` (/ _speed 1.75) _ball_2))))))

(event `InputAction|Exit`
  (params (Key :type "Key Structure"))
  ;[1 1 1] Clock Exit
  (:`Pressed`
    (`GameplayStatics.OpenLevel` "MainMenu")))

(fn `UserConstructionScript`)