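; Ball actor for a paddle game that waits on the player's paddle until launched, then moves at constant speed.
; While inactive it follows the player's Arrow component, and Launch applies an impulse and marks it active, which turns on the tail.
; Each tick its velocity is snapped to the nearest 45-degree diagonal at the set Speed.
; On destruction it reports a lost ball to the game mode and has the player spawn another.
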(event `self.ReceiveDestroyed`
  ;[1 1 1] Spawn new ball when this one is destroyed
  (`/Game/Blueprints/MyGameMode.LostBall` (`self.Game Mode`))
  (`/Game/Blueprints/Player_BP.Spawn New Ball` (`self.Player`)))

(event `self.ReceiveBeginPlay`
  ;[1 1 1] Get player
  (bind _asplayer_bp (cast `/Game/Blueprints/Player_BP` (`Controller.K2_GetPawn` (`GameplayStatics.GetPlayerController` 0))))
  (set `self.Player` _asplayer_bp)
  ;[1 1 1] Get Game Mode
  (bind _asmy_game_mode (cast `/Game/Blueprints/MyGameMode` (`GameplayStatics.GetGameMode`)))
  (set `self.Game Mode` _asmy_game_mode))

(event `self.ReceiveTick`
  (params (DeltaSeconds :type "Float (single-precision)"))
  (`self.Update Position`)
  (`self.Clamp Velocity`)
  (if (`self.Active`)
    (`ActorComponent.Activate` (`self.Tail`) false)))

(event `Launch`
  (params (Direction :type "Vector Structure"))
  ;[1 1 1] Launch ball
  (set `self.Active` true)
  (`PrimitiveComponent.AddImpulse` (`self.Ball`) Direction "None" true))

(event `Clamp Velocity`
  (bind _returnvalue (`KismetMathLibrary.MakeRotator` 0.0 0.0 45.0))
  (bind _speed (`self.Speed`))
  (bind _returnvalue_2 (`KismetMathLibrary.ClampVectorSize` (`self.GetVelocity`) _speed _speed))
  (bind (_returnvalue_roll _returnvalue_pitch _returnvalue_yaw) (`KismetMathLibrary.BreakRotator` (`KismetMathLibrary.MakeRotFromX` (`KismetMathLibrary.GreaterGreater_VectorRotator` _returnvalue_2 _returnvalue))))
  ;[1 1 1] Clamp Ball Velocity
  (`PrimitiveComponent.SetPhysicsLinearVelocity` (`self.Ball`) (* (`KismetMathLibrary.LessLess_VectorRotator` (`KismetMathLibrary.Conv_RotatorToVector` (`KismetMathLibrary.MakeRotator` 0.0 0.0 (`KismetMathLibrary.Conv_IntToDouble` (* (`KismetMathLibrary.Round` (/ _returnvalue_yaw 90.0)) 90)))) _returnvalue) (`KismetMathLibrary.VSize` _returnvalue_2)) false "None"))

(event `Update Position`
  (bind (_returnvalue_roll _returnvalue_pitch _returnvalue_yaw) (`KismetMathLibrary.BreakRotator` (`SceneComponent.K2_GetComponentRotation` (`self.Ball`))))
  ;[1 1 1] Attach to player paddle while not active
  (if (not (`self.Active`))
    (`self.K2_SetActorLocation` (`SceneComponent.K2_GetComponentLocation` (`/Game/Blueprints/Player_BP.Arrow` (`self.Player`))))
    ;[1 1 1] Set Tail rotation
    (`SceneComponent.K2_SetWorldRotation` (`self.Tail`) (`KismetMathLibrary.MakeRotator` 0.0 _returnvalue_pitch _returnvalue_yaw) false false)))

(fn `UserConstructionScript`)